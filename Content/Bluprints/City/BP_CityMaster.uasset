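; City actor that shows its name, gold, population and owner on a world widget, rotated each tick toward the camera pawn's camera.
; BeginPlay fills the widget and adds the city struct to the player controller's list, then sets Owner to the game instance's clan name.
; Hovering the widget shows a hand cursor.
; CallWidget uses a FlipFlop to alternately create and remove a CityDetail screen for this city.
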(event OnBeginCursorOver(Widget)
  (params (TouchedComponent :type Primitive%20Component%20Object%20Reference))
  (Variables|/Script/Engine.PlayerController|SetCurrentMouseCursor (Game|GetPlayerController 0) "Hand"))

(event OnEndCursorOver(Widget)
  (params (TouchedComponent :type Primitive%20Component%20Object%20Reference))
  (Variables|/Script/Engine.PlayerController|SetCurrentMouseCursor (Game|GetPlayerController 0) "None"))

(event Custom|Call%20Widget
  (Utilities|FlowControl|FlipFlop
    (:A
      (bind _returnvalue (UserInterface|CreateWidget "/Game/Bluprints/City/CityDetail.CityDetail_C" 0 (Variables|Default|GetCityInformation)))
      (bind _output_get (Variables|Default|SetCityWidget _returnvalue))
      (UserInterface|Viewport|AddtoViewport _output_get 0))
    (:B
      (Widget|RemovefromParent (Variables|Default|GetCityWidget)))))

(event EventTick
  (params (DeltaSeconds :type Float%20%28single-precision%29))
  (CallFunction|UpdatetoFace))

(event EventBeginPlay
  (bind _cityinformation (Variables|Default|GetCityInformation))
  (bind (_name _gold _population _owner) (Utilities|Struct|BreakCityStruct _cityinformation))
  (Utilities|FlowControl|Sequence
    (:then_0
      (bind _ascity_umg (Utilities|Casting|CastToCityUMG (UserInterface|GetUserWidgetObject (Variables|Default|GetWidget))))
      (Variables|/Game/Bluprints/City/CityUMG.CityUMG_C|SetName _ascity_umg _name)
      (Variables|/Game/Bluprints/City/CityUMG.CityUMG_C|SetGold _ascity_umg _gold)
      (Variables|/Game/Bluprints/City/CityUMG.CityUMG_C|Setpopulation _ascity_umg _population)
      (Variables|/Game/Bluprints/City/CityUMG.CityUMG_C|SetOwner _ascity_umg _owner))
    (:then_1
      (bind _asmy_player_controller (Utilities|Casting|CastToMyPlayerController (Game|GetPlayerController 0)))
      (bind _output_get (Variables|Default|SetPlayerControllerRef _asmy_player_controller))
      (Utilities|Array|Add (Variables|/Game/Bluprints/Character/MyPlayerController.MyPlayerController_C|GetCitys _output_get) (Variables|Default|GetCityInformation))
      (Utilities|Struct|SetmembersinCityStruct (Variables|Default|GetCityInformation) (Utilities|Struct|BreakClanStruct (Variables|/Game/Bluprints/MyGameInstance.MyGameInstance_C|GetClanStruct (.AsMy%20Game%20Instance (Utilities|Casting|CastToMyGameInstance (Game|GetGameInstance)))))))))

(fn ConstructionScript)

(fn UpdatetoFace
  (bind _ascamera_pawn (Utilities|Casting|CastToCameraPawn (Game|Player|GetPlayerPawn 0)))
  (Transformation|SetWorldRotation (Variables|Default|GetWidget) (Math|Rotator|FindLookatRotation (Transformation|GetWorldLocation (Variables|Default|GetWidget)) (Transformation|GetWorldLocation (Variables|/Game/Bluprints/Character/CameraPawn.CameraPawn_C|GetCamera _ascamera_pawn))) false false))